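; StartingWindow bootstraps the VR annotation session on BeginPlay: it opens a start dialog, quits if no path is chosen, and imports the selected LiDAR point cloud synchronously.
; LoadAndSpawnPointCloud configures the cloud actor's rendering, collision channel and classification colors, using defaults when dialog labels are too few.
; The actor stays hidden for the collision build call, avoiding failures on big clouds.
; It then spawns room, VR start and spectator, and signals import completion.
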(event EventBeginPlay
  (bind _original_point_cloud_coordinates (Variables|Default|GetOriginal%20Point%20Cloud%20Coordinates))
  (bind _minboundaries (Variables|Default|GetMinBoundaries))
  (bind _minboundaries_2 (Variables|Default|GetMinBoundaries))
  (bind (_x _y) (Math|Vector|BreakVector _original_point_cloud_coordinates))
  (bind _outfilename (Class|StartWindowActor|OpenStartWindow))
  (bind _output_get (Variables|Default|SetSelectedPath _outfilename))
  (if (Utilities|Array|IsEmpty _output_get)
    (Game|QuitGame (Game|GetPlayerController 0) "Quit" false)
    (else
      (bind _pointcloud (Class|LidarPointCloudBlueprintLibrary|CreatePointCloudfromFile (Variables|Default|GetSelectedPath) false)
        (:Success
          (bind _output_get_2 (Variables|Default|SetLoadedLidarPointCloud _pointcloud))
          (bind _returnvalue (Class|LidarPointCloud|GetClassificationsImported _output_get_2))
          (Variables|Default|SetNumberUniqueClassificationsImported (Utilities|Array|Length _returnvalue))
          (Variables|Default|SetClassificationColors (Class|StartWindowActor|GetClassificationColors)) ; Dialog Labels given
          (CallFunction|LoadandSpawnPointCloud)
          (Class|LidarPointCloud|BuildCollisionwithCallback (Variables|Default|GetLoadedLidarPointCloud))
          (Rendering|SetActorHiddenInGame (Variables|Default|GetLoadedLidarPointCloudActor) false) ; Has to be hidden before building collisions for big clouds, otherwise kaput
          (Game|SpawnActorfromClass "/Game/VRAnnotation/Blueprints/DynamicRoom.DynamicRoom_C" (Math|Transform|MakeTransform (Math|Vector|MakeVector _x _y (.Z (Math|Vector|BreakVector (Variables|Default|GetMinBoundaries)))) "0, 0, 0" "1.000000,1.000000,1.000000") "Undefined" "MultiplyWithRoot" 0 0)
          (Game|SpawnActorfromClass "/Script/VRExpansionPlugin.VRPlayerStart" (Math|Transform|MakeTransform (Math|Vector|MakeVector (.x _minboundaries_2) (.y _minboundaries_2) (.z _minboundaries_2)) (Math|Rotator|MakeRotator 0.0 0.0 (Class|KismetMathLibrary|DegAsin (Math|Float|SafeDivide (.x _minboundaries_2) (.y _minboundaries_2)))) "1.000000,1.000000,1.000000") "AlwaysSpawn" "MultiplyWithRoot" 0 0)
          (Game|SpawnActorfromClass "/Game/VRSpectator/VRSpectator.VRSpectator_C" (Math|Transform|MakeTransform (Math|Vector|MakeVector (.x _minboundaries) (.y _minboundaries) (.z _minboundaries)) (Math|Rotator|MakeRotator 0.0 0.0 (Class|KismetMathLibrary|DegAsin (Math|Float|SafeDivide (.x _minboundaries) (.y _minboundaries)))) "1.000000,1.000000,1.000000") "Undefined" "MultiplyWithRoot" 0 0)
          (Default|CallImportCompleted (Variables|Default|GetMinBoundaries) (Variables|Default|GetMaxBoundaries)))))))

(event Collision|EventActorBeginOverlap
  (params (OtherActor :type Actor%20Object%20Reference)))

(event EventTick
  (params (DeltaSeconds :type Float%20%28single-precision%29)))

(fn ConstructionScript)

(fn LoadandSpawnPointCloud
  (bind _loadedlidarpointcloud (Variables|Default|GetLoadedLidarPointCloud))
  (bind _returnvalue (Class|LidarPointCloud|GetBounds _loadedlidarpointcloud true))
  (bind (_min _max) (Utilities|Struct|BreakBox _returnvalue))
  (Variables|Default|SetOriginal%20Point%20Cloud%20Coordinates (Variables|/Script/LidarPointCloudRuntime.LidarPointCloud|GetOriginalCoordinates _loadedlidarpointcloud))
  (Variables|Default|SetMinBoundaries _min)
  (Variables|Default|SetMaxBoundaries _max)
  (bind _returnvalue_2 (Game|SpawnActorfromClass "/Script/LidarPointCloudRuntime.LidarPointCloudActor" (Math|Transform|MakeTransform (Variables|Default|GetOriginal%20Point%20Cloud%20Coordinates) "0, 0, 0" "1.000000,1.000000,1.000000") "AlwaysSpawn" "OverrideRootScale" 0 0))
  (Rendering|SetActorHiddenInGame _returnvalue_2 true) ; Has to be hidden before building collisions for big clouds, otherwise kaput
  (bind _output_get (Variables|Default|SetLoadedLidarPointCloudActor _returnvalue_2))
  (Variables|/Script/Engine.Actor|SetTags _output_get (Variables|Default|GetTags))
  (Variables|Default|SetLoadedPointCloudComponent (Actor|GetComponentbyClass _output_get "/Script/LidarPointCloudRuntime.LidarPointCloudComponent"))
  (Collision|SetCollisionObjectType (Variables|Default|GetLoadedPointCloudComponent) "ECC_GameTraceChannel2")
  (Class|LidarPointCloudComponent|SetPointCloud (Variables|Default|GetLoadedPointCloudComponent) (Variables|Default|GetLoadedLidarPointCloud))
  (Variables|/Script/LidarPointCloudRuntime.LidarPointCloudComponent|SetScalingMethod (Variables|Default|GetLoadedPointCloudComponent) "FixedScreenSize")
  (Variables|/Script/LidarPointCloudRuntime.LidarPointCloudComponent|SetPointSize (Variables|Default|GetLoadedPointCloudComponent) 0.15)
  (Class|LidarPointCloud|SetOptimizedforDynamicData (Variables|Default|GetLoadedLidarPointCloud) true)
  (Variables|/Script/LidarPointCloudRuntime.LidarPointCloudComponent|SetColorSource (Variables|Default|GetLoadedPointCloudComponent) "DataWithClassificationAlpha")
  (Variables|/Script/LidarPointCloudRuntime.LidarPointCloudComponent|SetbUseFrustumCulling (Variables|Default|GetLoadedPointCloudComponent) true)
  (if (<= (Variables|Default|GetNumberUniqueClassificationsImported) (Utilities|Map|Length (Variables|Default|GetClassificationColors))) ; If not enough, set default
    (Variables|/Script/LidarPointCloudRuntime.LidarPointCloudComponent|SetClassificationColors (Variables|Default|GetLoadedPointCloudComponent) (Variables|Default|GetClassificationColors))
    (else
      (Variables|/Script/LidarPointCloudRuntime.LidarPointCloudComponent|SetClassificationColors (Variables|Default|GetLoadedPointCloudComponent) (Variables|Default|GetDefaultClassificationColors))))
  (return))
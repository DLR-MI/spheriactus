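; VR tool actor for labelling and erasing LiDAR points with a right-hand spotlight, then exporting the result once the tutorial is completed.
; When DynamicRoom is ready, it loads labels and paths from StartWindowActor, spawns a target cloud and attaches a left-hand MVVM label panel.
; A self-calling zero-Delay event repeatedly runs SphereTraceCascade between original and target clouds.
; Inputs set label, radius, layers and color mode, or toggle the help diagram.
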(event Custom|ReadyForLabelling
  (bind _dynamicroom (Variables|Default|GetDynamicRoom))
  (bind _labelswidget (Variables|Default|GetLabelsWidget))
  (bind _listlabelscolor (Variables|/Game/VRAnnotation/UI/WBP_LabelsPanel.WBP_LabelsPanel_C|GetListLabelsColor _labelswidget))
  (bind _min_boundaries (Variables|/Game/VRAnnotation/Blueprints/DynamicRoom.DynamicRoom_C|GetMin%20Boundaries _dynamicroom))
  (bind _returnvalue (Actor|GetActorOfClass "/Game/Characters/VRCharacterCustom.VRCharacterCustom_C"))
  (bind _output_get (Variables|Default|SetVRCharacter _returnvalue))
  (Utilities|IsValid _output_get
    (:Is%20Valid
      (Class|VRBaseCharacter|SetActorLocationandRotationVR (Variables|Default|GetVRCharacter) (Math|Vector|MakeVector (.x _min_boundaries) (.y _min_boundaries) (.z _min_boundaries)) (Math|Rotator|MakeRotator 0.0 0.0 (Class|KismetMathLibrary|DegAsin (Math|Float|SafeDivide (.x _min_boundaries) (.y _min_boundaries)))) true true false true) ; In case VRPlayerStart won't work
      (Transformation|AttachComponentToComponent (Variables|Components|GetGrippableStaticMesh) (Variables|/Script/VRExpansionPlugin.VRBaseCharacter|GetRightMotionController (Variables|Default|GetVRCharacter)) "VRCharacterSocketRight" "KeepRelative" "KeepRelative" "KeepRelative" true)
      (bind _returnvalue_2 (Actor|GetActorOfClass "/Script/Spheriactus.StartWindowActor"))
      (bind _output_get_2 (Variables|Default|SetStartWindowActor _returnvalue_2))
      (Variables|Default|SetExportFilePath (Class|StartWindowActor|GetExportFilePath _output_get_2))
      (Variables|Default|SetImportFilePath (Class|StartWindowActor|GetImportFilePath _output_get_2))
      ;[1 1 1] Label Setting
      (bind _output_get_3 (Variables|Default|SetLabelEntries (Class|StartWindowActor|GetLabelEntries (Variables|Default|GetStartWindowActor))))
      (bind _keys (Utilities|Map|Keys _output_get_3))
      (bind _output_get_4 (Variables|Default|SetLabelNames _keys))
      (Variables|Default|SetCurrentLabelName (Utilities|Array|Get(acopy) _output_get_4))
      (bind _values (Utilities|Map|Values (Variables|Default|GetLabelEntries)))
      (bind _output_get_5 (Variables|Default|SetLabelColors _values))
      (Variables|Default|SetCurrentLabelColor (Utilities|Array|Get(acopy) _output_get_5))
      (Variables|Default|SetCurrentLabelIndex 0)
      (Variables|Default|SetTotalNumberOfLabels (Utilities|Map|Length (Variables|Default|GetLabelEntries)))
      (CallFunction|SetDiagramWidget)
      (CallFunction|SetupViewModel)
      (Class|ListView|SetSelectedItem _listlabelscolor (Class|ListView|GetItemat _listlabelscolor (Variables|Default|GetCurrentLabelIndex)))
      (Rendering|Components|Light|SetLightColor (Variables|Components|GetSpotLight) (Variables|Default|GetCurrentLabelColor) true)
      (bind _returnvalue_3 (Rendering|Material|CreateDynamicMaterialInstance (Variables|Components|GetGrippableStaticMesh) 0 0 "None" :!class /Script/Engine.PrimitiveComponent))
      (bind _output_get_6 (Variables|Default|SetMaterialInstancePCT _returnvalue_3))
      (Rendering|Material|SetVectorParameterValue _output_get_6 "PCTColor" (Variables|Default|GetCurrentLabelColor) :!class /Script/Engine.MaterialInstanceDynamic)
      (Rendering|Material|SetMaterial (Variables|Default|GetCylinderMesh) 0 (Variables|Default|GetMaterialInstancePCT))
      (Variables|Default|SetNumberOfLayers 0)
      (bind _outactors (Actor|GetAllActorsOfClasswithTag "/Script/LidarPointCloudRuntime.LidarPointCloudActor" "pointcloudloaded"))
      (for _array_element _outactors
        _)
      (bind _output_get_7 (Variables|Default|SetOriginalPointCloudActor _array_element))
      (Variables|Default|SetOriginalPointCloudActorTransform (Transformation|GetActorTransform _output_get_7))
      (bind _output_get_8 (Variables|Components|SetOriginalPointCloudComponent (Actor|GetComponentbyClass _output_get_7 "/Script/LidarPointCloudRuntime.LidarPointCloudComponent")))
      (bind _output_get_9 (Variables|Default|SetOriginalPointCloud (Class|LidarPointCloudActor|GetPointCloud (Variables|Default|GetOriginalPointCloudActor))))
      (Variables|Default|SetRadius 5.0)
      (Class|LidarPointCloud|SetOptimizedforDynamicData (Variables|Default|GetOriginalPointCloud) true)
      (bind _returnvalue_4 (Game|SpawnActorfromClass "/Script/LidarPointCloudRuntime.LidarPointCloudActor" (Variables|Default|GetOriginalPointCloudActorTransform) "AlwaysSpawn" "MultiplyWithRoot" 0 0))
      (bind _output_get_10 (Variables|Default|SetTargetedPointCloudActor _returnvalue_4))
      (bind _output_get_11 (Variables|Components|SetTargetedPointCloudComponent (Actor|GetComponentbyClass _output_get_10 "/Script/LidarPointCloudRuntime.LidarPointCloudComponent")))
      (Class|LidarPointCloudComponent|SetPointShape _output_get_11 "Circle")
      (Variables|/Script/LidarPointCloudRuntime.LidarPointCloudComponent|SetScalingMethod (Variables|Components|GetTargetedPointCloudComponent) "FixedScreenSize")
      (Variables|/Script/LidarPointCloudRuntime.LidarPointCloudComponent|SetPointSize (Variables|Components|GetTargetedPointCloudComponent) 0.4)
      (Class|LidarPointCloudComponent|SetPointCloud (Variables|Components|GetTargetedPointCloudComponent) (Class|LidarPointCloudBlueprintLibrary|CreatePointCloudEmpty))
      (bind _output_get_12 (Variables|Default|SetTargetedPointCloud (Class|LidarPointCloudActor|GetPointCloud (Variables|Default|GetTargetedPointCloudActor))))
      (Class|LidarPointCloud|SetOptimizedforDynamicData _output_get_12 true)
      (CallFunction|OnSphereTraceCompletion false))
    (:Is%20Not%20Valid
      (Game|QuitGame (Game|GetPlayerController 0) "Quit" false))))

(event Custom|OnSphereTraceCompletion
  (params (bLabel :type Boolean%20%28by%20ref%29) (CurrentLabelIndex :type Integer))
  (bind _spotlight (Variables|Components|GetSpotLight))
  (Utilities|FlowControl|Delay 0.0)
  (Class|SphereTraceCascade|SphereTraceCascade bLabel CurrentLabelIndex (Variables|Default|GetNumberOfLayers) (Variables|Default|GetRadius) (Transformation|GetWorldLocation _spotlight) (Math|Vector|GetForwardVector _spotlight) (Variables|Default|GetCurrentLabelColor) (Utilities|Array|MakeArray (Variables|Default|GetTargetedPointCloudActor) 0) (Utilities|Array|MakeArray "ObjectTypeQuery7") (Variables|Components|GetOriginalPointCloudComponent) (Variables|Components|GetTargetedPointCloudComponent) (Variables|Default|GetCylinderMesh))
  (bind _output_get (Variables|Default|SetLabellingInProgress false))
  (CallFunction|OnSphereTraceCompletion _output_get (Variables|Default|GetCurrentLabelIndex)))

(event Input|EnhancedActionEvents|EnhancedInputActionIA_Screenshot
  (params (ActionValue :type Boolean) (ElapsedSeconds :type Float%20%28double-precision%29) (TriggeredSeconds :type Float%20%28double-precision%29) (InputAction :type Input%20Action%20Object%20Reference :default "/Game/VRAnnotation/Input/Actions/IA_Screenshot.IA_Screenshot"))
  ;[1 1 1] Input for Screenshot
  (:Started
    (Development|ExecuteConsoleCommand "HighResShot 2" 0)))

(event Input|EnhancedActionEvents|EnhancedInputActionIA_Label
  (params (ActionValue :type Boolean) (ElapsedSeconds :type Float%20%28double-precision%29) (TriggeredSeconds :type Float%20%28double-precision%29) (InputAction :type Input%20Action%20Object%20Reference :default "/Game/VRAnnotation/Input/Actions/IA_Label.IA_Label"))
  ;[1 1 1] Input for Labelling Points v4
  (:Triggered
    (bind _output_get (Variables|Default|SetLabellingInProgress true :!label _label))
    (CallFunction|OnSphereTraceCompletion (and _output_get (Variables|Default|GetTutorialCompleted)) (Variables|Default|GetCurrentLabelIndex)))
  (:Started
    (goto _label)))

(event Input|EnhancedActionEvents|EnhancedInputActionIA_Radius_Scroll
  (params (ActionValue :type Float%20%28double-precision%29) (ElapsedSeconds :type Float%20%28double-precision%29) (TriggeredSeconds :type Float%20%28double-precision%29) (InputAction :type Input%20Action%20Object%20Reference :default "/Game/VRAnnotation/Input/Actions/IA_Radius_Scroll.IA_Radius_Scroll"))
  ;[1 1 1] Input For Changing Sphere Radius
  (if (and (>= (* (Variables|Default|GetRadius) (+ (* ActionValue 0.03) 1.0)) 1.0) (< (* (Variables|Default|GetRadius) (+ (* ActionValue 0.03) 1.0)) 25.0))
    (Variables|Default|SetRadius (* (Variables|Default|GetRadius) (+ (* ActionValue 0.03) 1.0)))
    (CallFunction|OnSphereTraceCompletion (Variables|Default|GetLabellingInProgress) (Variables|Default|GetCurrentLabelIndex))))

(event Input|EnhancedActionEvents|EnhancedInputActionIA_Layers_Scroll
  (params (ActionValue :type Float%20%28double-precision%29) (ElapsedSeconds :type Float%20%28double-precision%29) (TriggeredSeconds :type Float%20%28double-precision%29) (InputAction :type Input%20Action%20Object%20Reference :default "/Game/VRAnnotation/Input/Actions/IA_Layers_Scroll.IA_Layers_Scroll"))
  ;[1 1 1] Input For Changing Number of Layers
  (:Triggered
    (if true ; Added because of a bug in UE 5.5
      _))
  (:Started
    (Utilities|FlowControl|DelayUntilNextTick) ; Added because of a bug in UE 5.5
    (if (and (>= (+ (Variables|Default|GetNumberOfLayers) (Math|Float|Sign(Float) ActionValue)) 0) (< (+ (Variables|Default|GetNumberOfLayers) (Math|Float|Sign(Float) ActionValue)) 3))
      (Variables|Default|SetNumberOfLayers (+ (Variables|Default|GetNumberOfLayers) (Math|Float|Sign(Float) ActionValue)))
      (CallFunction|OnSphereTraceCompletion (Variables|Default|GetLabellingInProgress) (Variables|Default|GetCurrentLabelIndex)))))

(event Input|EnhancedActionEvents|EnhancedInputActionIA_Save_Labelled_Data
  (params (ActionValue :type Boolean) (ElapsedSeconds :type Float%20%28double-precision%29) (TriggeredSeconds :type Float%20%28double-precision%29) (InputAction :type Input%20Action%20Object%20Reference :default "/Game/VRAnnotation/Input/Actions/IA_Save_Labelled_Data.IA_Save_Labelled_Data"))
  ;[1 1 1] Input for Saving Labelled Point Cloud
  (if (Variables|Default|GetTutorialCompleted)
    (Class|LabellingDataManager|ExportLabelledPointCloudComponent (Variables|Components|GetOriginalPointCloudComponent) (Variables|Default|GetLabelNames) (Variables|Default|GetExportFilePath) (Variables|Default|GetImportFilePath))))

(event Input|EnhancedActionEvents|EnhancedInputActionIA_Label_Down
  (params (ActionValue :type Boolean) (ElapsedSeconds :type Float%20%28double-precision%29) (TriggeredSeconds :type Float%20%28double-precision%29) (InputAction :type Input%20Action%20Object%20Reference :default "/Game/VRAnnotation/Input/Actions/IA_Label_Down.IA_Label_Down"))
  (bind _labelswidget (Variables|Default|GetLabelsWidget))
  (bind _listlabelscolor (Variables|/Game/VRAnnotation/UI/WBP_LabelsPanel.WBP_LabelsPanel_C|GetListLabelsColor _labelswidget))
  ;[1 1 1] Input Action for going forward in the lable list
  (if (>= (+ (Variables|Default|GetCurrentLabelIndex) 1) (Variables|Default|GetTotalNumberOfLabels))
    (Variables|Default|SetCurrentLabelIndex 0)
    (else
      (bind _output_get (Variables|Default|SetCurrentLabelIndex (+ (Variables|Default|GetCurrentLabelIndex) 1)))))
  (Variables|Default|SetCurrentLabelName (Utilities|Array|Get(acopy) (Variables|Default|GetLabelNames) _output_get))
  (Variables|Default|SetCurrentLabelColor (Utilities|Array|Get(acopy) (Variables|Default|GetLabelColors) _output_get))
  (Rendering|Components|Light|SetLightColor (Variables|Components|GetSpotLight) (Variables|Default|GetCurrentLabelColor) true)
  (Rendering|Material|SetVectorParameterValue (Variables|Default|GetMaterialInstancePCT) "PCTColor" (Variables|Default|GetCurrentLabelColor) :!class /Script/Engine.MaterialInstanceDynamic)
  (Class|ListView|SetSelectedItem _listlabelscolor (Class|ListView|GetItemat _listlabelscolor (Variables|Default|GetCurrentLabelIndex))))

(event Input|EnhancedActionEvents|EnhancedInputActionIA_Label_Up
  (params (ActionValue :type Boolean) (ElapsedSeconds :type Float%20%28double-precision%29) (TriggeredSeconds :type Float%20%28double-precision%29) (InputAction :type Input%20Action%20Object%20Reference :default "/Game/VRAnnotation/Input/Actions/IA_Label_Up.IA_Label_Up"))
  (bind _labelswidget (Variables|Default|GetLabelsWidget))
  (bind _listlabelscolor (Variables|/Game/VRAnnotation/UI/WBP_LabelsPanel.WBP_LabelsPanel_C|GetListLabelsColor _labelswidget))
  ;[1 1 1] Input Action for going backward in the lable list
  (if (< (- (Variables|Default|GetCurrentLabelIndex) 1) 0)
    (bind _output_get (Variables|Default|SetCurrentLabelIndex (- (Variables|Default|GetTotalNumberOfLabels) 1)))
    (else
      (Variables|Default|SetCurrentLabelIndex (- (Variables|Default|GetCurrentLabelIndex) 1))))
  (Variables|Default|SetCurrentLabelName (Utilities|Array|Get(acopy) (Variables|Default|GetLabelNames) _output_get))
  (Variables|Default|SetCurrentLabelColor (Utilities|Array|Get(acopy) (Variables|Default|GetLabelColors) _output_get))
  (Rendering|Components|Light|SetLightColor (Variables|Components|GetSpotLight) (Variables|Default|GetCurrentLabelColor) true)
  (Rendering|Material|SetVectorParameterValue (Variables|Default|GetMaterialInstancePCT) "PCTColor" (Variables|Default|GetCurrentLabelColor) :!class /Script/Engine.MaterialInstanceDynamic)
  (Class|ListView|SetSelectedItem _listlabelscolor (Class|ListView|GetItemat _listlabelscolor (Variables|Default|GetCurrentLabelIndex))))

(event Input|EnhancedActionEvents|EnhancedInputActionIA_Undo_Label
  (params (ActionValue :type Boolean) (ElapsedSeconds :type Float%20%28double-precision%29) (TriggeredSeconds :type Float%20%28double-precision%29) (InputAction :type Input%20Action%20Object%20Reference :default "/Game/VRAnnotation/Input/Actions/IA_Undo_Label.IA_Undo_Label"))
  ;[1 1 1] Erase labelled data v2
  (:Triggered
    (bind _output_get (Variables|Default|SetLabellingInProgress true :!label _label))
    (CallFunction|OnSphereTraceCompletion _output_get -1))
  (:Started
    (goto _label)))

(event Input|EnhancedActionEvents|EnhancedInputActionIA_Show_Diagram
  (params (ActionValue :type Boolean) (ElapsedSeconds :type Float%20%28double-precision%29) (TriggeredSeconds :type Float%20%28double-precision%29) (InputAction :type Input%20Action%20Object%20Reference :default "/Game/VRAnnotation/Input/Actions/IA_Show_Diagram.IA_Show_Diagram"))
  ;[1 1 1] Toggle Diagram
  (:Started
    (if (Widget|IsVisible (Variables|Default|GetDiagramWidget))
      (Widget|SetVisibility (Variables|Default|GetDiagramWidget) "Collapsed")
      (if (not (Variables|Default|GetTutorialCompleted))
        (CallFunction|RunHeadsetTiltAnimation))
      (elif (not (Class|UserWidget|IsPlayingAnimation (Variables|Default|GetHeadsetAnimationWidget)))
        (Widget|SetVisibility (Variables|Default|GetDiagramWidget) "Visible")))))

(event Input|EnhancedActionEvents|EnhancedInputActionIA_Color_Mode_Change
  (params (ActionValue :type Boolean) (ElapsedSeconds :type Float%20%28double-precision%29) (TriggeredSeconds :type Float%20%28double-precision%29) (InputAction :type Input%20Action%20Object%20Reference :default "/Game/VRAnnotation/Input/Actions/IA_Color_Mode_Change.IA_Color_Mode_Change"))
  ;[1 1 1] Alternate between Color Sources
  (:Started
    (switch Utilities|FlowControl|Switch|SwitchonELidarPointCloudColorationMode (Variables|/Script/LidarPointCloudRuntime.LidarPointCloudComponent|GetColorSource (Variables|Components|GetOriginalPointCloudComponent))
      (:DataWithClassificationAlpha
        (Variables|/Script/LidarPointCloudRuntime.LidarPointCloudComponent|SetColorSource (Variables|Components|GetOriginalPointCloudComponent) "Classification"))
      (:Classification
        (Variables|/Script/LidarPointCloudRuntime.LidarPointCloudComponent|SetColorSource (Variables|Components|GetOriginalPointCloudComponent) "DataWithClassificationAlpha")))))

(event EventBeginPlay
  (bind _returnvalue (Actor|GetActorOfClass "/Game/VRAnnotation/Blueprints/DynamicRoom.DynamicRoom_C"))
  (bind _output_get (Variables|Default|SetDynamicRoom _returnvalue))
  (EventDispatchers|BindEventtoReadyforLabelling _output_get (delegate Custom|ReadyForLabelling)))

(event Input|KeyboardEvents|Right
  (params (Key :type Key%20Structure :default "None"))
  (bind _labelswidget (Variables|Default|GetLabelsWidget))
  (bind _listlabelscolor (Variables|/Game/VRAnnotation/UI/WBP_LabelsPanel.WBP_LabelsPanel_C|GetListLabelsColor _labelswidget))
  ;[1 1 1] Input Action for going forward in the lable list
  (:Pressed
    (if (>= (+ (Variables|Default|GetCurrentLabelIndex) 1) (Variables|Default|GetTotalNumberOfLabels))
      (Variables|Default|SetCurrentLabelIndex 0)
      (else
        (bind _output_get (Variables|Default|SetCurrentLabelIndex (+ (Variables|Default|GetCurrentLabelIndex) 1)))))
    (Variables|Default|SetCurrentLabelName (Utilities|Array|Get(acopy) (Variables|Default|GetLabelNames) _output_get))
    (Variables|Default|SetCurrentLabelColor (Utilities|Array|Get(acopy) (Variables|Default|GetLabelColors) _output_get))
    (Rendering|Components|Light|SetLightColor (Variables|Components|GetSpotLight) (Variables|Default|GetCurrentLabelColor) true)
    (Rendering|Material|SetVectorParameterValue (Variables|Default|GetMaterialInstancePCT) "PCTColor" (Variables|Default|GetCurrentLabelColor) :!class /Script/Engine.MaterialInstanceDynamic)
    (Class|ListView|SetSelectedItem _listlabelscolor (Class|ListView|GetItemat _listlabelscolor (Variables|Default|GetCurrentLabelIndex)))))

(event Input|KeyboardEvents|L
  (params (Key :type Key%20Structure :default "None"))
  ;[1 1 1] Input for Labelling Points v4
  (:Pressed
    (bind _output_get (Variables|Default|SetLabellingInProgress true))
    (CallFunction|OnSphereTraceCompletion (and _output_get (Variables|Default|GetTutorialCompleted)) (Variables|Default|GetCurrentLabelIndex))))

(event Input|KeyboardEvents|Add
  (params (Key :type Key%20Structure :default "None"))
  ;[1 1 1] Input For Changing Sphere Radius
  (:Pressed
    (Variables|Default|SetRadius (+ (Variables|Default|GetRadius) 1.0))
    (CallFunction|OnSphereTraceCompletion (Variables|Default|GetLabellingInProgress) (Variables|Default|GetCurrentLabelIndex))))

(event Input|KeyboardEvents|Subtract
  (params (Key :type Key%20Structure :default "None"))
  ;[1 1 1] Input For Changing Sphere Radius
  (:Pressed
    (Variables|Default|SetRadius (+ (Variables|Default|GetRadius) -1.0))
    (CallFunction|OnSphereTraceCompletion (Variables|Default|GetLabellingInProgress) (Variables|Default|GetCurrentLabelIndex))))

(event Input|KeyboardEvents|T
  (params (Key :type Key%20Structure :default "None"))
  ;[1 1 1] Input for Screenshot
  (:Pressed
    (Development|ExecuteConsoleCommand "HighResShot 2" 0)))

(event Input|KeyboardEvents|C
  (params (Key :type Key%20Structure :default "None"))
  ;[1 1 1] Alternate between Color Sources
  (:Pressed
    (switch Utilities|FlowControl|Switch|SwitchonELidarPointCloudColorationMode (Variables|/Script/LidarPointCloudRuntime.LidarPointCloudComponent|GetColorSource (Variables|Components|GetOriginalPointCloudComponent))
      (:DataWithClassificationAlpha
        (Variables|/Script/LidarPointCloudRuntime.LidarPointCloudComponent|SetColorSource (Variables|Components|GetOriginalPointCloudComponent) "Classification"))
      (:Classification
        (Variables|/Script/LidarPointCloudRuntime.LidarPointCloudComponent|SetColorSource (Variables|Components|GetOriginalPointCloudComponent) "DataWithClassificationAlpha")))))

(event Input|KeyboardEvents|U
  (params (Key :type Key%20Structure :default "None"))
  ;[1 1 1] Erase labelled data v2
  (:Pressed
    (bind _output_get (Variables|Default|SetLabellingInProgress true))
    (CallFunction|OnSphereTraceCompletion _output_get -1)))

(event Input|KeyboardEvents|Left
  (params (Key :type Key%20Structure :default "None"))
  (bind _labelswidget (Variables|Default|GetLabelsWidget))
  (bind _listlabelscolor (Variables|/Game/VRAnnotation/UI/WBP_LabelsPanel.WBP_LabelsPanel_C|GetListLabelsColor _labelswidget))
  ;[1 1 1] Input Action for going backward in the lable list
  (:Pressed
    (if (< (- (Variables|Default|GetCurrentLabelIndex) 1) 0)
      (bind _output_get (Variables|Default|SetCurrentLabelIndex (- (Variables|Default|GetTotalNumberOfLabels) 1)))
      (else
        (Variables|Default|SetCurrentLabelIndex (- (Variables|Default|GetCurrentLabelIndex) 1))))
    (Variables|Default|SetCurrentLabelName (Utilities|Array|Get(acopy) (Variables|Default|GetLabelNames) _output_get))
    (Variables|Default|SetCurrentLabelColor (Utilities|Array|Get(acopy) (Variables|Default|GetLabelColors) _output_get))
    (Rendering|Components|Light|SetLightColor (Variables|Components|GetSpotLight) (Variables|Default|GetCurrentLabelColor) true)
    (Rendering|Material|SetVectorParameterValue (Variables|Default|GetMaterialInstancePCT) "PCTColor" (Variables|Default|GetCurrentLabelColor) :!class /Script/Engine.MaterialInstanceDynamic)
    (Class|ListView|SetSelectedItem _listlabelscolor (Class|ListView|GetItemat _listlabelscolor (Variables|Default|GetCurrentLabelIndex)))))

(event Input|KeyboardEvents|B
  (params (Key :type Key%20Structure :default "None"))
  ;[1 1 1] Toggle Diagram
  (:Pressed
    (if (Widget|IsVisible (Variables|Default|GetDiagramWidget))
      (Widget|SetVisibility (Variables|Default|GetDiagramWidget) "Collapsed")
      (if (not (Variables|Default|GetTutorialCompleted))
        (CallFunction|RunHeadsetTiltAnimation))
      (elif (not (Class|UserWidget|IsPlayingAnimation (Variables|Default|GetHeadsetAnimationWidget)))
        (Widget|SetVisibility (Variables|Default|GetDiagramWidget) "Visible")))))

(event Input|KeyboardEvents|G
  (params (Key :type Key%20Structure :default "None"))
  ;[1 1 1] Input for Saving Labelled Point Cloud
  (:Pressed
    (if (Variables|Default|GetTutorialCompleted)
      (Class|LabellingDataManager|ExportLabelledPointCloudComponent (Variables|Components|GetOriginalPointCloudComponent) (Variables|Default|GetLabelNames) (Variables|Default|GetExportFilePath) (Variables|Default|GetImportFilePath)))))

(fn ConstructionScript)

(fn CalculateBoundingVolume
  (params (Min :type Vector) (Max :type Vector))
  (return (* (Math|Float|Absolute(Float) (- (.x Min) (.x Max))) (Math|Float|Absolute(Float) (- (.y Min) (.y Max))) (Math|Float|Absolute(Float) (- (.z Min) (.z Max))))))

(fn SetupViewModel
  (bind _returnvalue (Game|ConstructObjectfromClass "/Game/VRAnnotation/Viewmodels/VM_Labels.VM_Labels_C"))
  (bind _output_get (LocalVariables|SetVM_Labels _returnvalue))
  (Class|MVVMViewModelCollectionObject|AddViewModelInstance (Class|MVVMGameSubsystem|GetViewModelCollection (Subsystems|GetMVVMGameSubsystem)) (Utilities|Struct|MakeMVVMViewModelContext "/Game/VRAnnotation/Viewmodels/VM_Labels.VM_Labels_C" "VM_Labels") _output_get)
  (for (_array_element _array_index) (Variables|Default|GetLabelColors)
    (bind _returnvalue_2 (Game|ConstructObjectfromClass "/Game/VRAnnotation/Blueprints/DataHolderLabels.DataHolderLabels_C"))
    (Variables|/Game/VRAnnotation/Blueprints/DataHolderLabels.DataHolderLabels_C|SetStructureLabels _returnvalue_2 (Utilities|Struct|MakeStructureLabelsData (Utilities|Array|Get(acopy) (Variables|Default|GetLabelNames) _array_index) _array_element))
    (Utilities|Array|Add (Variables|Default|GetLabelData) _returnvalue_2))
  (Variables|/Game/VRAnnotation/Viewmodels/VM_Labels.VM_Labels_C|SetLabelData (LocalVariables|GetVM_Labels) (Variables|Default|GetLabelData))
  (bind _returnvalue_3 (UserInterface|CreateWidget "/Game/VRAnnotation/UI/WBP_LabelsPanel.WBP_LabelsPanel_C" (Game|GetPlayerController 0) (LocalVariables|GetVM_Labels)))
  (Variables|Default|SetLabelsWidget _returnvalue_3)
  (Class|ListView|SetListItems (Variables|/Game/VRAnnotation/UI/WBP_LabelsPanel.WBP_LabelsPanel_C|GetListLabelsColor (Variables|Default|GetLabelsWidget)) (Variables|Default|GetLabelData))
  (Class|ListView|SetListItems (Variables|/Game/VRAnnotation/UI/WBP_LabelsPanel.WBP_LabelsPanel_C|GetListLabelsName (Variables|Default|GetLabelsWidget)) (Variables|Default|GetLabelData))
  (bind _returnvalue_4 (AddComponent|AddWidgetComponent false (Math|Transform|MakeTransform "9.000000,0.500000,-5.000000" "105.000000,180.000000,0.000000" "0.020000,0.020000,0.020000")))
  (bind _output_get_2 (LocalVariables|SetLabelsWidgetComponent _returnvalue_4))
  (Class|WidgetComponent|SetWidgetSpace _output_get_2 "World")
  (UserInterface|SetWidget (LocalVariables|GetLabelsWidgetComponent) (Variables|Default|GetLabelsWidget))
  (Transformation|AttachComponentToComponent (LocalVariables|GetLabelsWidgetComponent) (Variables|/Script/VRExpansionPlugin.VRBaseCharacter|GetLeftMotionController (Variables|Default|GetVRCharacter)) "VRCharacterSocketLeft" "KeepRelative" "KeepRelative" "KeepRelative" true)
  (return))

(fn SetDiagramWidget
  (bind _returnvalue (UserInterface|CreateWidget "/Game/VRAnnotation/UI/WBP_DiagramScreen.WBP_DiagramScreen_C" (Game|GetPlayerController 0)))
  (Variables|Default|SetDiagramWidget _returnvalue)
  (bind _returnvalue_2 (AddComponent|AddVRStereoWidgetComponent false (Math|Transform|MakeTransform "70.000000,0.000000,-15.000000" "180.000000,0.000000,180.000000" "1.000000,1.000000,1.000000")))
  (bind _output_get (Variables|Default|SetDiagramWidgetComponent _returnvalue_2))
  (Class|WidgetComponent|SetWidgetSpace _output_get "World")
  (Class|WidgetComponent|SetDrawSize (Variables|Default|GetDiagramWidgetComponent) "(X=5000.000000,Y=5000.000000)")
  (UserInterface|SetWidget (Variables|Default|GetDiagramWidgetComponent) (Variables|Default|GetDiagramWidget))
  (Transformation|AttachComponentToComponent (Variables|Default|GetDiagramWidgetComponent) (Variables|/Script/VRExpansionPlugin.VRBaseCharacter|GetParentRelativeAttachment (Variables|Default|GetVRCharacter)) "VRCharacterCamera" "KeepRelative" "KeepRelative" "KeepWorld" false)
  (return))

(fn RunHeadsetTiltAnimation
  (Utilities|IsValid (Variables|Default|GetHeadsetAnimationWidget)
    (:Is%20Not%20Valid
      (bind _returnvalue (UserInterface|CreateWidget "/Game/VRAnnotation/UI/WBP_AnimatedHeadset.WBP_AnimatedHeadset_C" (Game|GetPlayerController 0)))
      (Variables|Default|SetHeadsetAnimationWidget _returnvalue)
      (bind _returnvalue_2 (AddComponent|AddVRStereoWidgetComponent false (Math|Transform|MakeTransform "70.000000,0.000000,-15.000000" "180.000000,0.000000,180.000000" "1.000000,1.000000,1.000000")))
      (bind _output_get (Variables|Default|SetHeadsetAnimationWidgetComponent _returnvalue_2))
      (Class|WidgetComponent|SetWidgetSpace _output_get "World")
      (Class|WidgetComponent|SetDrawSize (Variables|Default|GetHeadsetAnimationWidgetComponent) "(X=5000.000000,Y=5000.000000)")
      (UserInterface|SetWidget (Variables|Default|GetHeadsetAnimationWidgetComponent) (Variables|Default|GetHeadsetAnimationWidget))
      (Transformation|AttachComponentToComponent (Variables|Default|GetHeadsetAnimationWidgetComponent) (Variables|/Script/VRExpansionPlugin.VRBaseCharacter|GetParentRelativeAttachment (Variables|Default|GetVRCharacter)) "VRCharacterCamera" "KeepRelative" "KeepRelative" "KeepWorld" false)
      (return))))
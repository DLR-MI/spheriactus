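; DynamicRoom is a VR annotation actor that generates a room sized to imported data using Geometry Script.
; When StartingWindow reports import completion, it derives padded dimensions from the min and max bounds.
; It appends a rectangle, extrudes it by the height, adds a top rectangle and applies a translucent grid material.
; It then spawns the LabellingTool and calls ReadyForLabelling.
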(event Custom|ImportCompleted
  (params (MinBoundaries :type Vector) (MaxBoundaries :type Vector))
  (bind _output_get (Variables|Default|SetMin%20Boundaries MinBoundaries))
  (bind _output_get_2 (Variables|Default|SetMax%20Boundaries MaxBoundaries))
  (bind (_transformlocationx _transformlocationy _transformlocationz _dimensionx _dimensiony _dimensionz) (CallFunction|CalculateFloorBoundaries _output_get _output_get_2))
  (Variables|Default|SetDimension%20X _dimensionx)
  (Variables|Default|SetDimension%20Y _dimensiony)
  (Variables|Default|SetDimension%20Z _dimensionz)
  ;[1 1 1] Build Floors and Walls
  (bind _returnvalue (Class|GeometryScriptLibraryMeshPrimitiveFunctions|AppendRectangleXY :TargetMesh (Variables|Default|GetDynamicMesh) :Transform (Math|Transform|MakeTransform (Math|Vector|MakeVector 0.0 0.0 (* (Variables|Default|GetClearance) -1.0)) "0, 0, 0" "1.000000,1.000000,1.000000") :DimensionX (Variables|Default|GetDimension%20X) :DimensionY (Variables|Default|GetDimension%20Y) :Debug 0))
  (bind _returnvalue_2 (Class|GeometryScriptLibraryMeshModelingFunctions|ApplyMeshLinearExtrudeFaces :TargetMesh _returnvalue :Options (Utilities|Struct|MakeGeometryScriptMeshLinearExtrudeOptions (Variables|Default|GetDimension%20Z) "FixedDirection" "0.000000,0.000000,1.000000" "EntireSelection" (Utilities|Struct|MakeGeometryScriptMeshEditPolygroupOptions "PreserveExisting" 0) 1.0 true) :Debug 0))
  (bind _returnvalue_3 (Class|GeometryScriptLibraryMeshPrimitiveFunctions|AppendRectangleXY :TargetMesh _returnvalue_2 :Transform (Math|Transform|MakeTransform (Math|Vector|MakeVector 0.0 0.0 (- (Variables|Default|GetDimension%20Z) (Variables|Default|GetClearance))) "0, 0, 0" "1.000000,1.000000,1.000000") :DimensionX (Variables|Default|GetDimension%20X) :DimensionY (Variables|Default|GetDimension%20Y) :Debug 0))
  (Rendering|Material|SetMaterial (Variables|DynamicMeshActor|GetDynamicMeshComponent) 0 "/Game/VRAnnotation/Materials/TranslucentGrid.TranslucentGrid")
  (Game|SpawnActorfromClass "/Game/VRAnnotation/Blueprints/LabellingTool.LabellingTool_C" (Math|Transform|MakeTransform "11.000000,-1.000000,-5.000000" "-30.000000,0.000000,0.000000" "1.000000,1.000000,1.000000") "AlwaysSpawn" "MultiplyWithRoot" 0 0)
  (Default|CallReadyforLabelling))

(event EventBeginPlay
  (bind _returnvalue (Actor|GetActorOfClass "/Game/VRAnnotation/Blueprints/StartingWindow.StartingWindow_C"))
  (EventDispatchers|BindEventtoImportCompleted _returnvalue (delegate Custom|ImportCompleted)))

(event Collision|EventActorBeginOverlap
  (params (OtherActor :type Actor%20Object%20Reference)))

(event EventTick
  (params (DeltaSeconds :type Float%20%28single-precision%29)))

(fn ConstructionScript
  (bind _returnvalue (DynamicMeshComponent|GetDynamicMesh (Variables|DynamicMeshActor|GetDynamicMeshComponent)))
  (bind _returnvalue_2 (DynamicMesh|Reset _returnvalue))
  (Variables|Default|SetDynamicMesh _returnvalue_2))

(fn CalculateFloorBoundaries
  (params (MinBoundaries :type Vector) (MaxBoundaries :type Vector))
  (bind (_x _y _z) (Math|Vector|BreakVector MaxBoundaries))
  (bind (_x_2 _y_2 _z_2) (Math|Vector|BreakVector MinBoundaries))
  (return _x_2 _y (- (* (/ (+ _z_2 _z) 2.0) -1.0) 1.0) (+ (Math|Float|Absolute(Float) (- _x_2 _x)) 314.0) (+ (Math|Float|Absolute(Float) (- _y_2 _y)) 314.0) (+ (Math|Float|Absolute(Float) (- _z_2 _z)) 314.0)))

(fn EncasingwithColliders
  (params (Transform%20Location%20X :type Float%20%28double-precision%29) (Transform%20Location%20Y :type Float%20%28double-precision%29) (Transform%20Location%20Z :type Float%20%28double-precision%29) (Dimension%20X :type Float%20%28double-precision%29) (Dimension%20Y :type Float%20%28double-precision%29) (Dimension%20Z :type Float%20%28double-precision%29))
  (Class|GeometryScriptLibraryMeshPrimitiveFunctions|AppendBox :TargetMesh (Variables|Default|GetDynamicMesh) :Transform (Math|Transform|MakeTransform (Math|Vector|MakeVector 0.0 0.0 -1e+01) "0, 0, 0" "1.000000,1.000000,1.000000") :DimensionX Dimension%20X :DimensionY Dimension%20Y :DimensionZ 0.0 :Origin "Center" :Debug 0)
  (Rendering|Material|SetMaterial (Variables|DynamicMeshActor|GetDynamicMeshComponent) 0 "/Engine/EditorMaterials/PhAT_UnselectedMaterial.PhAT_UnselectedMaterial"))